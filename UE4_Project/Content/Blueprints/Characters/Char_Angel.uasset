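; Angel enemy character that chases the nearest player and kills any player it hits, through a server-side call to the game mode.
; PerceptionTick uses CanMove, which is not set here, and a DoOnce to issue one move toward the closest player, or to halt it in place.
; It also carries player-style input for movement, replicated running and camera-trace interaction via Interface_Interact, where interacted actors can capture yaw input.
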(event EventBeginPlay
  (CallFunction|InitializeMovement))

(event Collision|EventActorBeginOverlap
  (params (OtherActor :type Actor%20Object%20Reference)))

(event EventTick
  (params (DeltaSeconds :type Float%20%28single-precision%29))
  (CallFunction|TickInteract)
  (CallFunction|PerceptionTick))

(event Custom|Initialize%20Movement
  (Variables|/Script/Engine.CharacterMovementComponent|SetMaxWalkSpeed (Variables|Character|GetCharacterMovement) (Variables|Movement|GetWalkSpeed)))

(event Custom|Server%20Multi%20Run
  (params (Running :type Boolean))
  (bind _charactermovement (Variables|Character|GetCharacterMovement))
  ;[1 1 1] Running Trigger
  (if Running
    (Variables|/Script/Engine.CharacterMovementComponent|SetMaxWalkSpeed _charactermovement (Variables|Movement|GetRunSpeed))
    (else
      (Variables|/Script/Engine.CharacterMovementComponent|SetMaxWalkSpeed _charactermovement (Variables|Movement|GetWalkSpeed)))))

(event Custom|Server%20Run%20Trigger
  (params (Running :type Boolean))
  ;[1 1 1] Running Trigger
  (CallFunction|ServerMultiRun Running))

(event EventInputRun
  ;[1 1 1] Running Trigger
  (CallFunction|ServerRunTrigger true))

(event EventInputRunStop
  ;[1 1 1] Running Trigger
  (CallFunction|ServerRunTrigger false))

(event EventInputWalk
  (params (Axis :type Float%20%28single-precision%29))
  ;[1 1 1] Linear movement
  (if (Variables|Movement|GetCanMove)
    (Pawn|Input|AddMovementInput (Transformation|GetActorForwardVector) Axis false)))

(event EventInputStrafe
  (params (Axis :type Float%20%28single-precision%29))
  ;[1 1 1] Linear movement
  (if (Variables|Movement|GetCanMove)
    (Pawn|Input|AddMovementInput (Transformation|GetActorRightVector) Axis false)))

(event EventInputTurn
  (params (Axis :type Float%20%28single-precision%29))
  ;[1 1 1] Rotational Movement
  (if (Variables|Movement|GetCanMove)
    (if (Variables|Interaction|GetCaptureYaw)
      (Class|InterfaceInteract|InteractYaw(Message) (Variables|Interaction|GetInteract%20Actor) Axis)
      (else
        (Pawn|Input|AddControllerYawInput Axis)))))

(event EventInputPitch
  (params (Axis :type Float%20%28single-precision%29))
  ;[1 1 1] Rotational Movement
  (if (Variables|Movement|GetCanMove)
    (Pawn|Input|AddControllerPitchInput Axis)))

(event OnComponentHit(Mesh)
  (params (HitComponent :type Primitive%20Component%20Object%20Reference) (OtherActor :type Actor%20Object%20Reference) (OtherComp :type Primitive%20Component%20Object%20Reference) (NormalImpulse :type Vector :default "0, 0, 0") (Hit :type Hit%20Result%20Structure%20%28by%20ref%29))
  (Networking|SwitchHasAuthority
    (:Authority
      (bind _aschar_player (Utilities|Casting|CastToChar_Player OtherActor))
      (bind _asplayer_controller (Utilities|Casting|CastToPlayerController (Pawn|GetController _aschar_player)))
      (Default|PlayerDeath (.AsGM%20Game (Utilities|Casting|CastToGM_Game (Game|GetGameMode))) _asplayer_controller))))

(event Custom|Tick%20Interact
  (bind _camera (Variables|Default|GetCamera))
  (bind _returnvalue (Transformation|GetWorldLocation _camera))
  ;[1 1 1] Interact trace
  (bind (_outhit _returnvalue_2) (Collision|LineTraceByChannel _returnvalue (+ _returnvalue (* (Math|Vector|GetForwardVector _camera) (Variables|Interaction|GetInteract%20Distance))) "TraceTypeQuery1" false (Actor|GetAllChildActors true) "None"))
  (if _returnvalue_2
    (if (Utilities|DoesObjectImplementInterface (.HitActor (Collision|BreakHitResult _outhit)) "/Game/Blueprints/Interactable/Interface_Interact.Interface_Interact_C")
      (if (not (== (Variables|Interaction|GetInteract%20Actor) (.HitActor (Collision|BreakHitResult _outhit))))
        (bind _output_get (Variables|Interaction|SetInteract%20Actor (.HitActor (Collision|BreakHitResult _outhit))))
        (Class|InterfaceInteract|InteractBeginFocus(Message) _output_get)))
    (elif (not (Variables|Interaction|GetInteracting))
      (Class|InterfaceInteract|InteractEndFocus(Message) (Variables|Interaction|GetInteract%20Actor))
      (Variables|Interaction|SetInteract%20Actor 0))))

(event EventInputInteract
  (bind _interact_actor (Variables|Interaction|GetInteract%20Actor))
  ;[1 1 1] Interact trigger
  (Utilities|IsValid _interact_actor
    (:Is%20Valid
      (Variables|Interaction|SetInteracting true)
      (bind _capture_yaw (Class|InterfaceInteract|InteractBeginInteract(Message) _interact_actor (Pawn|GetController)))
      (Variables|Interaction|SetCaptureYaw _capture_yaw)
      (Class|InterfaceInteract|AngelBeginInteract(Message) _interact_actor))))

(event EventInputInteractStop
  (bind _interact_actor (Variables|Interaction|GetInteract%20Actor))
  ;[1 1 1] Interact trigger
  (Utilities|IsValid _interact_actor
    (:Is%20Valid
      (Variables|Interaction|SetInteracting false)
      (Class|InterfaceInteract|InteractEndInteract(Message) _interact_actor (Pawn|GetController))
      (Variables|Interaction|SetCaptureYaw false)
      (Class|InterfaceInteract|AngelEndInteract(Message) _interact_actor))))

(event Custom|Perception%20Tick
  (if (Variables|Movement|GetCanMove)
    (Utilities|IsValid (Variables|Perception|GetTarget)
      (:Is%20Valid
        _)
      (:Is%20Not%20Valid
        (Utilities|FlowControl|Sequence
          (:then_0
            _)
          (:then_1
            (goto _label Reset)))))
    (Utilities|FlowControl|DoOnce false :!label _label
      (:Completed
        (for _array_element (Variables|/Game/Blueprints/Modes_and_PCs/GM_Game.GM_Game_C|GetPlayers (.AsGM%20Game (Utilities|Casting|CastToGM_Game (Game|GetGameMode))))
          (Utilities|IsValid _array_element
            (:Is%20Valid
              (if (< (Math|Vector|VectorLength (- (Transformation|GetActorLocation _array_element) (Transformation|GetActorLocation))) (Variables|Perception|GetPlayerDistance))
                (Variables|Perception|SetPlayerDistance (Math|Vector|VectorLength (- (Transformation|GetActorLocation _array_element) (Transformation|GetActorLocation))))
                (Variables|Perception|SetTarget _array_element)))))
        (Variables|Perception|SetPlayerDistance 1e+09)
        (AI|Navigation|SimpleMovetoActor (Pawn|GetController) (Variables|Perception|GetTarget))
        (Development|PrintString "move" true true "(R=1.000000,G=0.000000,B=0.168417,A=1.000000)" 2e+01)))
    (else
      (Utilities|FlowControl|Sequence
        (:then_0
          (goto _label Reset))
        (:then_1
          (AI|Navigation|SimpleMovetoLocation (Pawn|GetController) (Transformation|GetActorLocation))
          (Development|PrintString "Stop Move" true true "(R=1.000000,G=0.548871,B=0.000000,A=1.000000)" 2e+01))))))

(fn ConstructionScript)