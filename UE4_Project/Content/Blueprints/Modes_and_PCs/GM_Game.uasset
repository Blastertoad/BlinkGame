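; Game mode for a Weeping Angels-style game: spawns players and Angels, freezes seen Angels, and moves dead players into Angel pawns.
; Each tick, non-blinking players check camera FOV, then socket-to-camera traces decide which Angels are seen.
; A timed loop traces from lit lights' arrow components to find lit Angels, the only candidates when a flashlight is off.
; An invalid player entry calls AngelsWin, which is an empty stub.
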(event EventBeginPlay
  (CallFunction|SpawnAngels)
  (CallFunction|PerceptionInitialize))

(event EventTick
  (params (DeltaSeconds :type Float%20%28single-precision%29))
  (CallFunction|PerceptionTick))

(event Custom|Spawn%20Angels
  ;[1 1 1] Spawn Angels and store in array
  (bind _outactors (Actor|GetAllActorsOfClass "/Game/Blueprints/Characters/Spawners/Spawn_Angel.Spawn_Angel_C"))
  (for _array_element _outactors
    (bind _returnvalue (Game|SpawnActorfromClass "/Game/Blueprints/Characters/Char_Angel.Char_Angel_C" (Transformation|GetActorTransform _array_element) "Undefined" 0 0))
    (Utilities|Array|Add (Variables|Default|GetAngels) _returnvalue)))

(event Custom|PlayerDeath
  (params (Controller :type Player%20Controller%20Object%20Reference))
  (bind _angels (Variables|Default|GetAngels))
  (Utilities|Array|Shuffle _angels)
  (for _array_element _angels
    (if (not (Pawn|IsPlayerControlled _array_element))
      (Actor|DestroyActor (Pawn|GetControlledPawn Controller))
      (Pawn|Possess Controller _array_element)
      (Variables|/Game/Blueprints/Characters/Char_Angel.Char_Angel_C|SetIsPlayer? _array_element true)
      (Development|PrintString "You died"))))

(event EventPostLogin
  (params (NewPlayer :type Player%20Controller%20Object%20Reference))
  ;[1 1 1] Spawn Players on login and store Pawns in array
  (bind _outactors (Actor|GetAllActorsOfClass "/Game/Blueprints/Characters/Spawners/Spawn_Player.Spawn_Player_C"))
  (bind _array_element (Utilities|Array|ForEachLoopwithBreak _outactors :!label _label)
    (:LoopBody
      (if (not (Variables|/Game/Blueprints/Characters/Spawners/Spawn_Player.Spawn_Player_C|GetUsed _array_element))
        (Variables|/Game/Blueprints/Characters/Spawners/Spawn_Player.Spawn_Player_C|SetUsed _array_element true)
        (bind _returnvalue (Game|SpawnActorfromClass "/Game/Blueprints/Characters/Char_Player.Char_Player_C" (Transformation|GetActorTransform _array_element) "Undefined" 0 0))
        (Pawn|Possess NewPlayer _returnvalue)
        (Utilities|Array|Add (Variables|Default|GetPlayers) _returnvalue)
        (goto _label Break)))))

(event Custom|Light%20Test
  ;[1 1 1] Clear previous results
  (Utilities|Array|Clear (Variables|Default|GetAngels%20In%20Light))
  ;[1 1 1] Check each light to see if it is on
  (for _array_element (Variables|Default|GetLighting)
    (if (Variables|/Game/Blueprints/Interactable/Class_Lighting.Class_Lighting_C|GetLightOn? _array_element)
      ;[1 1 1] If light is on run multiple ray traces to each Angel to see if it is hit light. If it is hit add to array of Angels in Light
      (for _array_element_2 (Actor|GetComponentsByClass _array_element "/Script/Engine.ArrowComponent")
        (for _array_element_3 (Variables|Default|GetAngels)
          (bind (_outhit _returnvalue) (Collision|LineTraceByChannel (Transformation|GetWorldLocation _array_element_2) (Transformation|GetActorLocation _array_element_3) "TraceTypeQuery1" false 0 "None"))
          (if _returnvalue
            (if (== _array_element_3 (.HitActor (Collision|BreakHitResult _outhit)))
              (Utilities|Array|AddUnique (Variables|Default|GetAngels%20In%20Light) _array_element_3))))))))

(event Custom|Set%20Angels%20Seen
  ;[1 1 1] Go through all Angels and set if they are seen or not.
  (for _array_element (Variables|Default|GetAngels)
    (if (Utilities|Array|ContainsItem (Variables|Default|GetAngelsSeen) _array_element)
      (Variables|/Game/Blueprints/Characters/Char_Angel.Char_Angel_C|SetCanMove _array_element false)
      (else
        (Variables|/Game/Blueprints/Characters/Char_Angel.Char_Angel_C|SetCanMove _array_element true)))))

(event Custom|Perception%20Initialize
  ;[1 1 1] Get all lighting objects in level
  (bind _outactors (Actor|GetAllActorsOfClass "/Game/Blueprints/Interactable/Class_Lighting.Class_Lighting_C"))
  (Variables|Default|SetLighting _outactors)
  ;[1 1 1] Start loop
  (CallFunction|LightingLoop))

(event Custom|Lighting%20Loop
  ;[1 1 1] Custom looping timer instead of tick.
  (Utilities|FlowControl|Sequence
    (:then_0
      (goto _label Open))
    (:then_1
      (Utilities|FlowControl|Gate true :!label _label
        (:Exit
          (Utilities|FlowControl|Sequence
            (:then_0
              (Utilities|FlowControl|Delay (Variables|Default|GetPerception%20Timer))
              (goto _label))
            (:then_1
              (CallFunction|LightTest))))))))

(event Custom|Perception%20Tick
  ;[1 1 1] Clear list of visible Angels
  (Utilities|Array|Clear (Variables|Default|GetAngelsSeen))
  ;[1 1 1] Go through each player. Can they see? Is their flashlight on?
  (for _array_element (Variables|Default|GetPlayers)
    (Utilities|IsValid _array_element
      (:Is%20Valid
        (if (not (Variables|/Game/Blueprints/Characters/Char_Player.Char_Player_C|GetBlinking? _array_element))
          ;[1 1 1] Is this angel in the player's feild of view. FOV adjusted for mesh size.
          (for _array_element_2 (select (Variables|/Game/Blueprints/Characters/Char_Player.Char_Player_C|GetFlashlight _array_element) (Variables|Default|GetAngels) (Variables|Default|GetAngels%20In%20Light))
            (if (< (Class|KismetMathLibrary|DegAcos (Math|Vector|DotProduct (Math|Vector|Normalize (Math|Vector|GetForwardVector (Math|Rotator|FindLookatRotation (Transformation|GetActorLocation _array_element) (Transformation|GetActorLocation _array_element_2)))) (Math|Vector|Normalize (Math|Vector|GetForwardVector (Variables|/Game/Blueprints/Characters/Char_Player.Char_Player_C|GetCamera _array_element))))) (+ (Variables|PlayerPerception|GetFOV%20adjust) (/ (Variables|/Script/Engine.CameraComponent|GetFieldOfView (Variables|/Game/Blueprints/Characters/Char_Player.Char_Player_C|GetCamera _array_element)) 2.0)))
              ;[1 1 1] If angel is in field of view do a line trace from mesh sockets back to player to see if they have line of sight
              (for _array_element_3 (Transformation|GetAllSocketNames (Variables|/Script/Engine.Character|GetMesh _array_element_2))
                (bind (_outhit _returnvalue) (Collision|LineTraceByChannel (Transformation|GetSocketLocation (Variables|/Script/Engine.Character|GetMesh _array_element_2) _array_element_3) (Transformation|GetWorldLocation (Variables|/Game/Blueprints/Characters/Char_Player.Char_Player_C|GetCamera _array_element)) "TraceTypeQuery1" false (Variables|Default|GetAngels) "None"))
                (if _returnvalue
                  (if (== _array_element (.HitActor (Collision|BreakHitResult _outhit)))
                    (Utilities|Array|AddUnique (Variables|Default|GetAngelsSeen) _array_element_2))))))))
      (:Is%20Not%20Valid
        ;[1 1 1] If there are no valid players the Angel team wins
        (CallFunction|AngelsWin))))
  (CallFunction|SetAngelsSeen))

(event Custom|Angels%20Win)

(fn ConstructionScript)