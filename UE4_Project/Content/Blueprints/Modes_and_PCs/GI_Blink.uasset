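; GI_Blink, apparently the game instance, handles hosting and joining multiplayer sessions through Advanced Sessions nodes, with a LAN option.
; HostGame creates a five-connection session, then opens the test map as a listen server.
; When split screen is enabled, hosting also adds a second local player, hides the first player's cursor and sets game-only input.
; JoinGame searches for sessions with a free slot and joins the first result.
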(event Custom|JoinGame
  (bind _returnvalue (Game|GetPlayerController 0))
  (bind _results (|FindSessionsAdvanced _returnvalue 0 (Variables|Networking|GetLan) "AllServers" 0 false false false 1)
    (:OnSuccess
      (|JoinSession _returnvalue (Utilities|Array|Get(acopy) _results)))))

(event Custom|HostGame
  (bind _returnvalue (Game|GetPlayerController 0))
  (|AdvancedSession 0 (Game|GetPlayerController 0) 5 0 (Variables|Networking|GetLan) true false true true false false false true
    (:OnSuccess
      (Game|OpenLevel(byName) "Map_Test" true "listen")
      (if (Variables|Input|GetSplitScreen)
        (Class|GameplayStatics|CreatePlayer 1)
        (Variables|/Script/Engine.PlayerController|SetbShowMouseCursor _returnvalue false)
        (Input|SetInputModeGameOnly _returnvalue)))))