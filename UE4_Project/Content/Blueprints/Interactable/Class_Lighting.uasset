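; Interactable light actor that shows or hides its point light according to the LightOn flag.
; On BeginPlay it line traces from each of eight arrow components to the actor's origin, ignoring the parent actor, and destroys obstructed arrows; the arrows serve as trace components in the game mode.
; Tick polls LightOn, using paired DoOnce nodes that reset each other so visibility is set only when the state changes.
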(event EventBeginPlay
  ;[1 1 1] Cycle trough arrows (used as trace components in game mode) and line trace to origin. If obstructed destroy component.
  (for _array_element (Utilities|Array|MakeArray (Variables|Default|GetArrow) (Variables|Default|GetArrow2) (Variables|Default|GetArrow3) (Variables|Default|GetArrow4) (Variables|Default|GetArrow5) (Variables|Default|GetArrow6) (Variables|Default|GetArrow1) (Variables|Default|GetArrow7))
    (bind _returnvalue (Collision|LineTraceByChannel (Transformation|GetWorldLocation _array_element) (Transformation|GetActorLocation) "TraceTypeQuery1" false (Utilities|Array|MakeArray (Actor|GetParentActor)) "None"))
    (if _returnvalue
      (Components|DestroyComponent _array_element))))

(event EventTick
  (params (DeltaSeconds :type Float%20%28single-precision%29))
  (bind _pointlight (Variables|Default|GetPointLight))
  (if (Variables|Default|GetLightOn?)
    (Utilities|FlowControl|Sequence
      (:then_0
        (Utilities|FlowControl|DoOnce false :!label _label
          (:Completed
            (Rendering|SetVisibility _pointlight true false))))
      (:then_1
        (goto _label_2 Reset)))
    (else
      (Utilities|FlowControl|Sequence
        (:then_0
          (Utilities|FlowControl|DoOnce false :!label _label_2
            (:Completed
              (Rendering|SetVisibility _pointlight false false))))
        (:then_1
          (goto _label Reset))))))

(fn ConstructionScript)