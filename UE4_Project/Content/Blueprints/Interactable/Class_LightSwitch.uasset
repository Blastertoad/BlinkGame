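; Interactable light switch that toggles every Class_Lighting actor sharing its LinkID.
; Ending an interaction calls ServerTrigger, which relays to MultiCastSwitchLights, named as a server-to-multicast replication chain.
; The switch event searches all lighting actors and inverts LightOn on each match, so it keeps no state of its own.
; Begin interact does nothing and returns false.
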(event Custom|Server%20Trigger
  (CallFunction|MultiCastSwitchLights))

(event Custom|MultiCast%20Switch%20Lights
  (bind _outactors (Actor|GetAllActorsOfClass "/Game/Blueprints/Interactable/Class_Lighting.Class_Lighting_C"))
  (for _array_element _outactors
    (if (== (Variables|/Game/Blueprints/Interactable/Class_Lighting.Class_Lighting_C|GetLinkID _array_element) (Variables|Default|GetLink_ID))
      (Variables|/Game/Blueprints/Interactable/Class_Lighting.Class_Lighting_C|SetLightOn? _array_element (select (Variables|/Game/Blueprints/Interactable/Class_Lighting.Class_Lighting_C|GetLightOn? _array_element) false true)))))

(event EventInteractEndInteract
  (params (Controller :type Controller%20Object%20Reference))
  (CallFunction|ServerTrigger))

(fn ConstructionScript)

(fn InteractBeginInteract
  (params (Controller :type Controller%20Object%20Reference))
  (return false))