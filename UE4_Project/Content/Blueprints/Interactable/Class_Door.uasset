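; Door Blueprint that the player swings open and shut by feeding a yaw axis while interacting with it.
; Begin interact always accepts the controller.
; Each yaw input rotates the Hinge component by a scaled amount, provided the hinge's current yaw plus the raw axis stays within a quarter turn to either side.
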(event EventInteractYaw
  (params (Axis :type Float%20%28single-precision%29))
  (bind _hinge (Variables|Default|GetHinge))
  (bind _relativerotation (Variables|/Script/Engine.SceneComponent|GetRelativeRotation _hinge))
  (bind _returnvalue (+ (.yaw _relativerotation) Axis))
  (if (and (< _returnvalue 9e+01) (> _returnvalue -9e+01))
    (Transformation|AddRelativeRotation _hinge (Math|Rotator|MakeRotator 0.0 0.0 (* Axis 2.5)) false false)))

(fn ConstructionScript)

(fn InteractBeginInteract
  (params (Controller :type Controller%20Object%20Reference))
  (return true))